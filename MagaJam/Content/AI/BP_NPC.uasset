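; BP_NPC is an enemy that endlessly chases the player character and damages it on capsule overlap, limited by a short cooldown.
; It registers in the game mode's living-enemy count on BeginPlay and re-issues AIMoveTo after each success or failure.
; Lethal damage decrements that count, triggers a remaining-enemy check, awards the player score and destroys the NPC.
; The perception handler is empty, with its tag-based chase logic left disconnected.
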(event OnTargetPerceptionUpdated(AIPerception)
  (params (Actor :type Actor%20Object%20Reference) (Stimulus :type AI%20Stimulus%20Structure))
  ;[1 1 1] Have to implement "Player" tag in thirdpersoncharac
)

(event OnComponentBeginOverlap(Capsule)
  (params (OverlappedComponent :type Primitive%20Component%20Object%20Reference) (OtherActor :type Actor%20Object%20Reference) (OtherComp :type Primitive%20Component%20Object%20Reference) (OtherBodyIndex :type Integer) (bFromSweep :type Boolean) (SweepResult :type Hit%20Result%20Structure%20%28by%20ref%29))
  (if (Variables|Default|GetcanAttack)
    (bind _asbp_third_person_character (Utilities|Casting|CastToBP_ThirdPersonCharacter OtherActor))
    (Variables|/Game/ThirdPerson/Blueprints/BP_ThirdPersonCharacter.BP_ThirdPersonCharacter_C|SetHealth _asbp_third_person_character (- (Variables|/Game/ThirdPerson/Blueprints/BP_ThirdPersonCharacter.BP_ThirdPersonCharacter_C|GetHealth _asbp_third_person_character) 2e+01))
    (Variables|Default|SetcanAttack false)
    (Utilities|FlowControl|Delay 2.0)
    (Variables|Default|SetcanAttack true)))

(event Custom|ChasePlayer
  (bind _asbp_third_person_character (Utilities|Casting|CastToBP_ThirdPersonCharacter (Game|GetPlayerCharacter 0)))
  (AI|AIMoveTo self "0, 0, 0" _asbp_third_person_character 5e+01 false
    (:OnSuccess
      _)
    (:OnFail
      _))
  (CallFunction|ChasePlayer))

(event EventBeginPlay
  (bind _asbp_third_person_game_mode (Utilities|Casting|CastToBP_ThirdPersonGameMode (Game|GetGameMode)))
  (Math|Integer|IncrementInt (Variables|/Game/ThirdPerson/Blueprints/BP_ThirdPersonGameMode.BP_ThirdPersonGameMode_C|GetEnemyAlive _asbp_third_person_game_mode)
    (:%20%20
      (bind _asbp_third_person_character (Utilities|Casting|CastToBP_ThirdPersonCharacter (Game|GetPlayerCharacter 0)))
      (AI|AIMoveTo self "0, 0, 0" _asbp_third_person_character 5e+01 false
        (:OnSuccess
          _)
        (:OnFail
          _))
      (CallFunction|ChasePlayer))))

(event Game|Damage|EventAnyDamage
  (params (Damage :type Float%20%28single-precision%29) (DamageType :type Damage%20Type%20Object%20Reference) (InstigatedBy :type Controller%20Object%20Reference) (DamageCauser :type Actor%20Object%20Reference))
  (bind _output_get (Variables|Default|SetHealth (- (Variables|Default|GetHealth) Damage)))
  (if (<= _output_get 0.0)
    (bind _asbp_third_person_game_mode (Utilities|Casting|CastToBP_ThirdPersonGameMode (Game|GetGameMode)))
    (Math|Integer|DecrementInt (Variables|/Game/ThirdPerson/Blueprints/BP_ThirdPersonGameMode.BP_ThirdPersonGameMode_C|GetEnemyAlive _asbp_third_person_game_mode)
      (:%20%20
        (Default|CheckEnemyLeft _asbp_third_person_game_mode)
        (Utilities|FlowControl|Sequence
          (:then_0
            (bind _asbp_third_person_character (Utilities|Casting|CastToBP_ThirdPersonCharacter (Game|GetPlayerCharacter 0)))
            (Default|GainScore _asbp_third_person_character (Variables|Default|GetNPC_ScorePoint)))
          (:then_1
            (Actor|DestroyActor)))))))

(fn ConstructionScript)